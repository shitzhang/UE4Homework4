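; BP_Objective is a damageable objective actor that awards score to players who hit it.
; Every tick it moves to the objective center plus offset read from MyGameState, so the game state drives its position.
; Any damage event increments the score on the instigator's MyPlayerState, regardless of the damage amount.
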(event EventTick
  (params (DeltaSeconds :type Float%20%28single-precision%29))
  (bind _asmy_game_state (Utilities|Casting|CastToMyGameState (Game|GetGameState)))
  (Transformation|SetActorLocation (+ (Variables|/Game/Blueprints/MyGameState.MyGameState_C|GetObjectiveCenter _asmy_game_state) (Variables|/Game/Blueprints/MyGameState.MyGameState_C|GetOffset _asmy_game_state)) false false))

(event Collision|EventActorBeginOverlap
  (params (OtherActor :type Actor%20Object%20Reference)))

(event Game|Damage|EventAnyDamage
  (params (Damage :type Float%20%28single-precision%29) (DamageType :type Damage%20Type%20Object%20Reference) (InstigatedBy :type Controller%20Object%20Reference) (DamageCauser :type Actor%20Object%20Reference))
  (bind _asmy_player_state (Utilities|Casting|CastToMyPlayerState (Variables|/Script/Engine.Controller|GetPlayerState InstigatedBy)))
  (Default|IncrementScore _asmy_player_state))

(fn ConstructionScript)
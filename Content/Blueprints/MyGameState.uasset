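; Game state Blueprint that runs a match countdown, resets player scores and triggers the game over menu.
; SetTimer decrements LeftTime through a looping one-second Delay, then calls ShowGameOverMenu on player controller 0 when it runs out.
; ClearPlayerScore zeroes PlayerScore across PlayerArray, while Tick computes a sine/cosine circular Offset in the XZ plane from elapsed time.
; Both OnRep functions are empty.
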(event Custom|ShowGameOver
  (bind _asmy_player_controller (Utilities|Casting|CastToMyPlayerController (Game|GetPlayerController 0)))
  (Default|ShowGameOverMenu _asmy_player_controller))

(event Custom|SetTimer
  (Utilities|FlowControl|Delay 1.0 :!label _label)
  (bind _result (Math|Integer|DecrementInt (Variables|Default|GetLeftTime))
    (:%20%20
      (if (<= _result 0)
        (CallFunction|ShowGameOver)
        (else
          (goto _label))))))

(event Custom|ClearPlayerScore
  (for _array_element (Variables|Default|GetPlayerArray self)
    (bind _asmy_player_state (Utilities|Casting|CastToMyPlayerState _array_element))
    (Variables|/Game/Blueprints/MyPlayerState.MyPlayerState_C|SetPlayerScore _asmy_player_state 0)))

(event EventTick
  (params (DeltaSeconds :type Float%20%28single-precision%29))
  (bind _movementradius (Variables|Default|GetMovementRadius))
  (bind _output_get (Variables|Default|SetElapseTime (+ (Variables|Default|GetElapseTime) DeltaSeconds)))
  (Variables|Default|SetOffset (Math|Vector|MakeVector (* (Math|Trig|Sin(Radians) (* _output_get (Variables|Default|GetTimeScale))) _movementradius) 0.0 (* _movementradius (Math|Trig|Cos(Radians) (* _output_get (Variables|Default|GetTimeScale)))))))

(fn ConstructionScript)

(fn OnRepGameStartTimer)

(fn OnRepRandomTimerValue1)